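; Third-person shooter player character Blueprint with aim zoom and mouse look.
; The Aim input plays a Zoom timeline forward or in reverse, lerping the spring arm length from its BeginPlay value to that value minus ZoomModifier.
; Look inputs turn the controller and feed aim-offset variables through Server-named events, sending control-to-actor pitch delta but a constant zero for yaw.
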(event `self.ReceiveBeginPlay`
  (set `self.Initial Target Arm Length` (`SpringArmComponent.TargetArmLength` (`self.SpringArmComponent`))))

(event `InputAction|Aim`
  (params (Key :type "Key Structure"))
  (bind _initial_target_arm_length (`self.Initial Target Arm Length`))
  (:`Pressed`
    (bind (_direction _newtrack_0) (`Timeline|Zoom` :!via `PlayFromStart` :!label _label)
      (:`Update`
        (set `SpringArmComponent.TargetArmLength` (`KismetMathLibrary.Lerp` _initial_target_arm_length (- _initial_target_arm_length (`self.ZoomModifier`)) _newtrack_0) (`self.SpringArmComponent`)))))
  (:`Released`
    (goto _label :!via `ReverseFromEnd`)))

(event `self.ReceiveTick`
  (params (DeltaSeconds :type "Float (single-precision)")))

(event `InputAxis|TurnAround`
  (params (AxisValue :type "Float (single-precision)"))
  ;[1 1 1] AimOffset Replication
  (`self.TurnAroundServer` 0.0)
  (`self.AddControllerYawInput` AxisValue))

(event `InputAxis|LookUp`
  (params (AxisValue :type "Float (single-precision)"))
  (bind (_returnvalue_roll _returnvalue_pitch) (`KismetMathLibrary.BreakRotator` (`KismetMathLibrary.NormalizedDeltaRotator` (`self.GetControlRotation`) (`self.K2_GetActorRotation`))))
  ;[1 1 1] AimOffset Replication
  (`self.LookUpServer` _returnvalue_pitch)
  (`self.AddControllerPitchInput` AxisValue))

(event `LookUpServer`
  (params (LookUpAxis :type "Float (double-precision)"))
  ;[1 1 1] AimOffset Replication
  (set `self.LookUpAxis` LookUpAxis))

(event `TurnAroundServer`
  (params (`Turn Around Axis` :type "Float (double-precision)"))
  ;[1 1 1] AimOffset Replication
  (set `self.Turn Around Axis` `Turn Around Axis`))

(fn `OnRep_ZoomModifier`)

(fn `UserConstructionScript`)